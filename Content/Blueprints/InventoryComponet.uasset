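; An inventory slot collision component that takes InventoryCube actors released from a motion controller.
; On overlap it stores one held cube as GrabActor, skipping cubes held by ControllertoIgnore when that is set, and clears it when that cube leaves.
; Tick watches the stored cube and, while no controller holds it, attaches it to the component, snapping location and rotation while keeping world scale.
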(event `self.ReceiveBeginPlay`
  (add `self.OnComponentBeginOverlap` (delegate `BeginOverlap`))
  (add `self.OnComponentEndOverlap` (delegate `EndOverlap`)))

(event `BeginOverlap` :!signature `self.OnComponentBeginOverlap`
  (params (OverlappedComponent :type "PrimitiveComponent Object Reference") (OtherActor :type "Actor Object Reference") (OtherComp :type "PrimitiveComponent Object Reference") (OtherBodyIndex :type Integer) (bFromSweep :type Boolean) (SweepResult :type "HitResult Structure (by ref)"))
  (bind _controllertoignore (`self.ControllertoIgnore`))
  (`/Engine/EditorBlueprintResources/StandardMacros.IsValid` (`self.GrabActor`)
    (:`Is Not Valid`
      (bind _asinventory_cube (cast `/Game/Blueprints/InventoryCube` OtherActor))
      (bind _motion_controller (`/Game/Blueprints/InventoryCube.Motion Controller` _asinventory_cube))
      (`/Engine/EditorBlueprintResources/StandardMacros.IsValid` _motion_controller
        (:`Is Valid`
          (`/Engine/EditorBlueprintResources/StandardMacros.IsValid` _controllertoignore
            (:`Is Valid`
              (if (!= _controllertoignore _motion_controller)
                (set `self.GrabActor` _asinventory_cube :!label _label)))
            (:`Is Not Valid`
              (goto _label))))))))

(event `EndOverlap`
  (params (OverlappedComponent :type "PrimitiveComponent Object Reference") (OtherActor :type "Actor Object Reference") (OtherComp :type "PrimitiveComponent Object Reference") (OtherBodyIndex :type Integer))
  (if (== OtherActor (`self.GrabActor`))
    (set `self.GrabActor` null)))

(event `self.ReceiveTick`
  (params (DeltaSeconds :type "Float (single-precision)"))
  (bind _grabactor (`self.GrabActor`))
  (`/Engine/EditorBlueprintResources/StandardMacros.IsValid` _grabactor
    (:`Is Valid`
      (`/Engine/EditorBlueprintResources/StandardMacros.IsValid` (`/Game/Blueprints/InventoryCube.Motion Controller` _grabactor)
        (:`Is Not Valid`
          (`Actor.K2_AttachToComponent` _grabactor self "None" "SnapToTarget" "SnapToTarget" "KeepWorld" true))))))